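; HexSpawn is a construction-script Blueprint that lays out a grid of random tile meshes, such as grass, forest, house and dirt.
; It loops over Rows and Cols, adding a static mesh component per cell and shifting alternate rows by Offset for a staggered hex layout.
; Each cell picks a mesh from a hardcoded array, where repeated Grass entries weight the odds.
; The event graph is unused.
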(fn `UserConstructionScript`
  (bind _output_get (set `self.tiles` (`|MakeArray` "/Game/Tiles/Dirt/grass.grass" "/Game/Tiles/Dirt/grass_forest.grass_forest" "/Game/Tiles/Dirt/grass.grass" "/Game/Buildings/Full_Buildings/building_house.building_house" "/Game/Tiles/Dirt/dirt.dirt" :!type "StaticMesh Object Reference")))
  (for _index (range (+ (`self.rows`) 1))
    (for _index_2 (range (+ (`self.cols`) 1))
      (bind _returnvalue (* _index (`self.spacingX`)))
      (bind _returnvalue_2 (* _index_2 (`self.spacingY`)))
      (bind _returnvalue_3 (`AddComponent|NODE_AddStaticMeshComponent-0` :`RelativeTransform` (`KismetMathLibrary.MakeTransform` (`KismetMathLibrary.SelectVector` (`KismetMathLibrary.MakeVector` (`KismetMathLibrary.Conv_IntToDouble` _returnvalue) (`KismetMathLibrary.Conv_IntToDouble` _returnvalue_2)) (`KismetMathLibrary.MakeVector` (`KismetMathLibrary.Conv_IntToDouble` _returnvalue) (`KismetMathLibrary.Conv_IntToDouble` (+ (`self.offset`) _returnvalue_2))) (== (mod _index 2) 0)) (struct) (0.0 0.0 0.0))))
      (`StaticMeshComponent.SetStaticMesh` _returnvalue_3 (`|GetArrayItem` (`self.tiles`) (`KismetMathLibrary.RandomInteger` (`KismetArrayLibrary.Array_Length` _output_get))))
      (`SceneComponent.SetWorldScale3D` _returnvalue_3 (`KismetMathLibrary.MakeVector` 1.0 1.0 (`KismetMathLibrary.RandomFloatInRange` 1.0 1.0))))))